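; Player camera pawn that pans, zooms and rotates in 45-degree steps.
; Input events only update desired location, rotation and clamped spring arm length, with movement following the actor's forward and right vectors.
; Tick interpolates the actor transform and arm length toward those targets for smooth motion, without sweep collision.
; Pan and zoom add a fixed step per input event, not scaled by delta time.
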(event EventTick
  (params (DeltaSeconds :type Float%20%28single-precision%29))
  (bind _springarm (Variables|Default|GetSpringArm))
  (Variables|/Script/Engine.SpringArmComponent|SetTargetArmLength _springarm (Math|Interpolation|FInterpTo (Variables|/Script/Engine.SpringArmComponent|GetTargetArmLength _springarm) (Variables|Default|GetZoom_Desired) DeltaSeconds 1e+01))
  (Transformation|SetActorLocation (Math|Interpolation|VInterpTo (Transformation|GetActorLocation) (Variables|Default|GetLocation_Desired) DeltaSeconds 5.0) false false)
  (Transformation|SetActorRotation (Math|Interpolation|RInterpTo (Transformation|GetActorRotation) (Variables|Default|GetRotation_Desired) DeltaSeconds 5.0)))

(event EventBeginPlay
  (Variables|Default|SetZoom_Desired (Variables|/Script/Engine.SpringArmComponent|GetTargetArmLength (Variables|Default|GetSpringArm)))
  (Variables|Default|SetLocation_Desired (Transformation|GetActorLocation))
  (Variables|Default|SetRotation_Desired (Transformation|GetActorRotation)))

(event Input|ActionEvents|InputActionInputAction_RotationRight
  (params (Key :type Key%20Structure :default "None"))
  (:Pressed
    (Variables|Default|SetRotation_Desired (Math|Rotator|CombineRotators (Variables|Default|GetRotation_Desired) "0.000000,-45.000000,0.000000"))))

(event Input|ActionEvents|InputActionInpitAction_RotationLeft
  (params (Key :type Key%20Structure :default "None"))
  (:Pressed
    (Variables|Default|SetRotation_Desired (Math|Rotator|CombineRotators (Variables|Default|GetRotation_Desired) "0.000000,45.000000,0.000000"))))

(event Input|AxisEvents|InputAxisInputAxis_Zoom
  (params (AxisValue :type Float%20%28single-precision%29))
  (Variables|Default|SetZoom_Desired (Math|Float|Clamp(Float) (+ (Variables|Default|GetZoom_Desired) (* AxisValue 2e+02)) 3e+02 2e+03)))

(event Input|AxisEvents|InputAxisInputAxis_Right
  (params (AxisValue :type Float%20%28single-precision%29))
  (Variables|Default|SetLocation_Desired (+ (Variables|Default|GetLocation_Desired) (* (* AxisValue 4e+01) (Transformation|GetActorRightVector)))))

(event Input|AxisEvents|InputAxisInputAxis_Forward
  (params (AxisValue :type Float%20%28single-precision%29))
  (Variables|Default|SetLocation_Desired (+ (Variables|Default|GetLocation_Desired) (* (* AxisValue 4e+01) (Transformation|GetActorForwardVector)))))

(fn ConstructionScript)